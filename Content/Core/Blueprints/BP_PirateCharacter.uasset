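; BP_PirateCharacter is the pirate character Blueprint, handling touch-screen camera look and a fire input.
; A touch press splits the viewport at its horizontal midpoint, and right-side drags feed frame-to-frame deltas, scaled by SenX and SenY, into controller yaw and pitch.
; Left-side drags only print a debug string.
; IA_Fire sets IsFiring when ammo is non-zero and the character is neither firing nor reloading.
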(event `InputTouch`
  (params (Location :type "Vector Structure") (FingerIndex :type "ETouchIndex Enum"))
  (bind _returnvalue (`KismetMathLibrary.MakeVector2D` Location_X Location_Y))
  ; Input Touch Logic
  (:`Pressed`
    (if (< (/ (`PlayerController.GetViewportSize` (`GameplayStatics.GetPlayerController` 0)) 2) (`KismetMathLibrary.FTrunc` Location_X))
      (set `self.Is Right Side` true)
      (set `self.TouchStartPosition` _returnvalue)
      (else
        (set `self.Is Right Side` false))))
  (:`Moved`
    (if (`self.Is Right Side`)
      (bind _output_get (set `self.TouchCurrentPosition` _returnvalue))
      (bind (_returnvalue_x _returnvalue_y) (`KismetMathLibrary.BreakVector2D` (- _output_get (`self.TouchStartPosition`))))
      (`self.AddControllerYawInput` (* _returnvalue_x (`self.SenX`)))
      (`self.AddControllerPitchInput` (* _returnvalue_y (`self.SenY`)))
      (set `self.TouchStartPosition` (`self.TouchCurrentPosition`))
      (else
        (`KismetSystemLibrary.PrintString` "Is Left Side")))))

(event `EnhancedInput|/Game/Core/Inputs/Actions/IA_Fire`
  (params (ActionValue :type Boolean) (ElapsedSeconds :type "Float (double-precision)") (TriggeredSeconds :type "Float (double-precision)") (InputAction :type "InputAction Object Reference" :default "/Game/Core/Inputs/Actions/IA_Fire.IA_Fire"))
  (:`Triggered`
    (if (and (!= (`self.current Ammo`) 0) (not (`self.Is Firing ?`)) (not (`self.Is Reloading`)))
      (set `self.Is Firing ?` true))))

(fn `UserConstructionScript`
  (`parent.UserConstructionScript`))